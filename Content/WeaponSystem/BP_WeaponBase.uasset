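; BP_WeaponBase is a base weapon Blueprint that handles firing and attachment to a character.
; WeaponFire plays the firing animation on the skeletal mesh and spawns a BP_Projectile at the mesh's barrel socket transform, regardless of collision.
; AttachToHand and AttachToHolster snap the weapon to the given character's mesh at the HandSocket or HolsterSocket variable.
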(event Custom|Weapon%20Fire
  (bind _skeletalmesh (Variables|Default|GetSkeletalMesh))
  (bind _returnvalue (Transformation|GetSocketTransform _skeletalmesh "barrel" "RTS_World"))
  (Components|Animation|PlayAnimation (Variables|Default|GetSkeletalMesh) (Variables|Default|GetFiringAnim) false)
  (Game|SpawnActorfromClass "/Game/WeaponSystem/BP_Projectile.BP_Projectile_C" (Math|Transform|MakeTransform (.location _returnvalue) (.rotation _returnvalue) (.scale _returnvalue)) "AlwaysSpawn" "MultiplyWithRoot" 0 0))

(event Custom|AttachToHolster
  (params (CharToAttach :type BP%20Third%20Person%20Character%20Object%20Reference))
  (Transformation|AttachComponentToComponent (Variables|/Script/Engine.Character|GetMesh CharToAttach) (Variables|Default|GetHolsterSocket) "SnapToTarget" "SnapToTarget" "SnapToTarget" true))

(event Custom|AttachToHand
  (params (CharToAttach :type BP%20Third%20Person%20Character%20Object%20Reference))
  (Transformation|AttachComponentToComponent (Variables|/Script/Engine.Character|GetMesh CharToAttach) (Variables|Default|GetHandSocket) "SnapToTarget" "SnapToTarget" "SnapToTarget" true))

(fn ConstructionScript)